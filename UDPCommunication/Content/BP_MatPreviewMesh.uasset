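; A preview mesh actor whose transform and material color are driven by data received through the UDP communication game mode.
; On BeginPlay it caches the game mode and creates a dynamic material instance.
; Each tick it polls the transform and color protocols, applies fresh data to the mesh or "Color" parameter, then clears that protocol, printing transforms.
; The Sender input sends default transform data through the game mode.
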(event `self.ReceiveBeginPlay`
  (bind _asudpcommunication_game_mode (cast `UDPCommunicationGameMode` (`GameplayStatics.GetGameMode`)))
  (set `self.GameMode` _asudpcommunication_game_mode)
  (bind _returnvalue (`PrimitiveComponent.CreateDynamicMaterialInstance` (`self.StaticMeshComponent`) 0 null))
  (set `self.DynamicMaterialInstance` _returnvalue))

(event `self.ReceiveTick`
  (params (DeltaSeconds :type "Float (single-precision)"))
  (`|ExecutionSequence`
    (:`then_0`
      (bind (_data _returnvalue) (`NetworkProtocolTransform.GetLatest` (`UDPCommunicationGameMode.GetTransformProtocol` (`self.GameMode`))))
      (if _returnvalue
        (`SceneComponent.K2_SetRelativeTransform` (`self.StaticMeshComponent`) (`KismetMathLibrary.MakeTransform` (break `TransformData` _data) (`.Rotation` (break `TransformData` _data)) (`.Scale` (break `TransformData` _data))) false false)
        (`NetworkProtocolTransform.Clear` (`UDPCommunicationGameMode.GetTransformProtocol` (`self.GameMode`)))
        (`KismetSystemLibrary.PrintString` (`KismetStringLibrary.Conv_VectorToString` (break `TransformData` _data)))
        (`KismetSystemLibrary.PrintString` (`KismetStringLibrary.Conv_RotatorToString` (`.Rotation` (break `TransformData` _data))))
        (`KismetSystemLibrary.PrintString` (`KismetStringLibrary.Conv_VectorToString` (`.Scale` (break `TransformData` _data))))))
    (:`then_1`
      (bind (_data_2 _returnvalue_2) (`NetworkProtocolColor.GetLatest` (`UDPCommunicationGameMode.GetColorProtocol` (`self.GameMode`))))
      (if _returnvalue_2
        (`MaterialInstanceDynamic.SetVectorParameterValue` (`self.DynamicMaterialInstance`) "Color" (break `ColorData` _data_2))
        (`NetworkProtocolColor.Clear` (`UDPCommunicationGameMode.GetColorProtocol` (`self.GameMode`)))))))

(event `InputAction|Sender`
  (params (Key :type "Key Structure" :default "AnyKey"))
  (:`Pressed`
    (`UDPCommunicationGameMode.Send` (`self.GameMode`) (make `TransformData` (0.0 0.0 0.0)))))

(fn `UserConstructionScript`)